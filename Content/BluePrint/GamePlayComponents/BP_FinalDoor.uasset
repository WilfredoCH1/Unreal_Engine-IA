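; BP_FinalDoor is a door actor that opens once every collectable item in the level has been collected.
; On BeginPlay it counts all BP_CollectableItem actors and opens immediately if there are none.
; Its ItemCollected event decrements that remaining count and opens the door when it reaches zero.
; Opening simply destroys the door actor, with no animation.
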(event Custom|openDoo
  (Actor|DestroyActor))

(event Custom|ItemCollected
  (bind _result (Math|Integer|DecrementInt (Variables|Default|GetRemainingCollectableItem))
    (:%20%20
      (if (== _result 0)
        (CallFunction|OpenDoo)))))

(event EventBeginPlay
  (bind _outactors (Actor|GetAllActorsOfClass "/Game/BluePrint/GamePlayComponents/BP_CollectableItem.BP_CollectableItem_C"))
  (bind _output_get (Variables|Default|SetRemainingCollectableItem (Utilities|Array|Length _outactors)))
  (if (== _output_get 0)
    (CallFunction|OpenDoo)))

(event Collision|EventActorBeginOverlap
  (params (OtherActor :type Actor%20Object%20Reference)))

(event EventTick
  (params (DeltaSeconds :type Float%20%28single-precision%29)))

(fn ConstructionScript)